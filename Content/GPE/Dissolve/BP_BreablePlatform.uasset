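; Breakable platform that dissolves when damaged by an enemy bullet.
; Construction applies the configurable mesh and a fixed material, and BeginPlay passes that mesh to the BPC_Dissolve component, which handles the dissolve.
; Mesh hits play a tremble sound and a Timeline-driven tilt, gated by a DoOnce that resets when the Timeline finishes.
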(event `self.ReceiveBeginPlay`
  ;[1 0 0.02009 0.5] Essential Setup for BPC_Dissolve
  (`/Game/GPE/Dissolve/BPC_Dissolve.SetUp` (`self.BPC_Disolve`) (`StaticMeshComponent.StaticMesh` (`self.StaticMesh`))))

(event `OnHit`
  ;[1 0 0.02009 0.5] Custom event to run dissolve !! Deactivates collison and view in game automatically
)

(event `self.ReceiveAnyDamage`
  (params (Damage :type "Float (single-precision)") (DamageType :type "DamageType Object Reference") (InstigatedBy :type "Controller Object Reference") (DamageCauser :type "Actor Object Reference"))
  (if (== (`GameplayStatics.GetObjectClass` DamageCauser) "/Game/GPE/BP_EnemyBullet.BP_EnemyBullet_C")
    (`/Game/GPE/Dissolve/BPC_Dissolve.Dissolve` (`self.BPC_Disolve`))))

(event `self.StaticMesh.OnComponentHit`
  (params (HitComponent :type "PrimitiveComponent Object Reference") (OtherActor :type "Actor Object Reference") (OtherComp :type "PrimitiveComponent Object Reference") (NormalImpulse :type "Vector Structure") (Hit :type "HitResult Structure (by ref)"))
  (`/Engine/EditorBlueprintResources/StandardMacros.DoOnce` false :!label _label
    (:`Completed`
      (`GameplayStatics.PlaySoundAtLocation` "/Game/Import/SFX/Environment/PlatformTremble.PlatformTremble" (`self.K2_GetActorLocation`) (struct) 0.7 1.0 0.0 null null null null)
      (bind (_direction _newtrack_0) (`Timeline|Timeline`)
        (:`Update`
          (`SceneComponent.K2_SetRelativeRotation` (`self.StaticMesh`) (`KismetMathLibrary.RLerp` (struct) (struct :`Roll` 3.0) _newtrack_0 true) false false))
        (:`Finished`
          (goto _label :!via `Reset`))))))

(fn `UserConstructionScript`
  (bind _staticmesh (`self.StaticMesh`))
  (`StaticMeshComponent.SetStaticMesh` _staticmesh (`self.BP Mesh`))
  (`PrimitiveComponent.SetMaterial` _staticmesh 0 "/Game/Fab/Megascans/Surfaces/Rock_Cliff_xccibbi/Medium/xccibbi_tier_2/Materials/MI_xccibbi.MI_xccibbi"))