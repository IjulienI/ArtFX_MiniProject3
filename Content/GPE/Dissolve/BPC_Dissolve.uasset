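; BPC_Dissolve is a component that temporarily replaces its owning actor with a Niagara dissolve effect.
; SetUp stores the static mesh, which Dissolve passes to a spawned NS_DisR system before hiding the owner and disabling its collision.
; A looping timer feeds the player's location to the effect and prints it.
; After the loop duration, the effect and timer are cleared and the owner's visibility and collision return.
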(event `Dissolve`
  (bind _returnvalue (`self.GetOwner`))
  (bind _returnvalue_2 (`self.GetOwner`))
  (bind _loopduration (`self.LoopDuration`))
  (`Actor.SetActorEnableCollision` _returnvalue false)
  (bind _returnvalue_3 (`NiagaraFunctionLibrary.SpawnSystemAtLocation` "/Game/GPE/Dissolve/NS_DisR.NS_DisR" (`Actor.K2_GetActorLocation` _returnvalue) (`Actor.K2_GetActorRotation` _returnvalue) (1.0 1.0 1.0) true false))
  (bind _output_get (set `self.MyNiagraSystem` _returnvalue_3))
  (`NiagaraFunctionLibrary.OverrideSystemUserVariableStaticMesh` (`self.MyNiagraSystem`) "Static Mesh" (`self.StaticMesh`))
  (`NiagaraComponent.SetVariableFloat` _output_get "Loop Duration" _loopduration)
  (`NiagaraComponent.SetVariableFloat` (`self.MyNiagraSystem`) "Loop Duration" _loopduration)
  (`self.Activate` (`self.MyNiagraSystem`) false)
  (bind _returnvalue_4 (`KismetSystemLibrary.K2_SetTimerDelegate` (delegate `RelayPlayerLocation`) 0.05 true))
  (set `self.TimerEvent` _returnvalue_4)
  (`Actor.SetActorHiddenInGame` _returnvalue true)
  (`KismetSystemLibrary.Delay` _loopduration)
  (`self.K2_DestroyComponent` (`self.MyNiagraSystem`))
  (`KismetSystemLibrary.K2_ClearAndInvalidateTimerHandle` (`self.TimerEvent`))
  (`Actor.SetActorEnableCollision` _returnvalue_2 true)
  (`Actor.SetActorHiddenInGame` _returnvalue_2 false))

(event `RelayPlayerLocation`
  (bind _returnvalue (`Actor.K2_GetActorLocation` (`GameplayStatics.GetPlayerPawn` 0)))
  (`KismetSystemLibrary.PrintString` (`KismetStringLibrary.Conv_VectorToString` _returnvalue) true true (struct :`G` 0.66 :`B` 1.0 :`A` 1.0) 0.1)
  (`NiagaraComponent.SetVariableVec3` (`self.MyNiagraSystem`) "PlayerLoc" _returnvalue))

(fn `SetUp`
  (params (NewParam :type "StaticMesh Object Reference"))
  (set `self.StaticMesh` NewParam))