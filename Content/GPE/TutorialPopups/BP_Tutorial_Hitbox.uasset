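; BP_Tutorial_Hitbox is a trigger volume that shows a tutorial popup for a movement or combat mechanic while the player stands inside it.
; On BeginPlay, each instance creates its own WBP_Tutorial widget and adds it to the viewport.
; When the player pawn enters the Hitbox, ENUMTutorialState selects which widget panel becomes visible.
; When the player pawn leaves, all tutorial panels in that widget are hidden.
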(event `self.ReceiveBeginPlay`
  ;[0.1999 1 0.1667 0.5] Begin Play
  (bind _returnvalue (`|CreateWidget` "/Game/GPE/TutorialPopups/WBP_Tutorial.WBP_Tutorial_C"))
  (bind _output_get (set `self.Widget_REF` _returnvalue))
  (`UserWidget.AddToViewport` _returnvalue 0)
  (`UserWidget.AddToViewport` _output_get 0))

(event `self.Hitbox.OnComponentBeginOverlap`
  (params (OverlappedComponent :type "PrimitiveComponent Object Reference") (OtherActor :type "Actor Object Reference") (OtherComp :type "PrimitiveComponent Object Reference") (OtherBodyIndex :type Integer) (bFromSweep :type Boolean) (SweepResult :type "HitResult Structure (by ref)"))
  (bind _widget_ref (`self.Widget_REF`))
  ;[1 0.1615 0.4527 0.5] Player Triggers Overlap
  (if (== OtherActor (`GameplayStatics.GetPlayerPawn` 0))
    (switch `/Game/GPE/TutorialPopups/ENUM_Tutorial` (`self.ENUM_TutorialState`)
      (:`NewEnumerator0`
        (`Widget.SetVisibility` (`/Game/GPE/TutorialPopups/WBP_Tutorial.VB_DoubleJump` _widget_ref) "Visible"))
      (:`NewEnumerator1`
        (`Widget.SetVisibility` (`/Game/GPE/TutorialPopups/WBP_Tutorial.VB_Dash` _widget_ref) "Visible"))
      (:`NewEnumerator2`
        (`Widget.SetVisibility` (`/Game/GPE/TutorialPopups/WBP_Tutorial.VB_Run` _widget_ref) "Visible"))
      (:`NewEnumerator3`
        (`Widget.SetVisibility` (`/Game/GPE/TutorialPopups/WBP_Tutorial.VB_Wallrun` _widget_ref) "Visible"))
      (:`NewEnumerator4`
        (`Widget.SetVisibility` (`/Game/GPE/TutorialPopups/WBP_Tutorial.VB_Glide` _widget_ref) "Visible"))
      (:`NewEnumerator5`
        (`Widget.SetVisibility` (`/Game/GPE/TutorialPopups/WBP_Tutorial.VB_Combo` _widget_ref) "Visible")))))

(event `self.Hitbox.OnComponentEndOverlap`
  (params (OverlappedComponent :type "PrimitiveComponent Object Reference") (OtherActor :type "Actor Object Reference") (OtherComp :type "PrimitiveComponent Object Reference") (OtherBodyIndex :type Integer))
  ;[1 0.1615 0.4527 0.5] Player Triggers Overlap
  (if (== OtherActor (`GameplayStatics.GetPlayerPawn` 0))
    (`Widget.SetVisibility` (`/Game/GPE/TutorialPopups/WBP_Tutorial.VB_DoubleJump` (`self.Widget_REF`)) "Hidden")
    (`Widget.SetVisibility` (`/Game/GPE/TutorialPopups/WBP_Tutorial.VB_Run` (`self.Widget_REF`)) "Hidden")
    (`Widget.SetVisibility` (`/Game/GPE/TutorialPopups/WBP_Tutorial.VB_Dash` (`self.Widget_REF`)) "Hidden")
    (`Widget.SetVisibility` (`/Game/GPE/TutorialPopups/WBP_Tutorial.VB_Wallrun` (`self.Widget_REF`)) "Hidden")
    (`Widget.SetVisibility` (`/Game/GPE/TutorialPopups/WBP_Tutorial.VB_Glide` (`self.Widget_REF`)) "Hidden")
    (`Widget.SetVisibility` (`/Game/GPE/TutorialPopups/WBP_Tutorial.VB_Combo` (`self.Widget_REF`)) "Hidden")))

(fn `UserConstructionScript`)