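; BP_EnemyBullet is an enemy projectile that deals damage and spawns fireflies where it lands.
; On BeginPlay a timeline lerps it unswept from its spawn point to FinalLocation, using the data asset's ProjectileFXDuration as play rate.
; On arrival, a small debug-drawn sphere trace picks the actor to damage.
; It then scatters a fixed or random number of BP_Firefly actors, passing on BossPhase, and destroys itself.
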(event `self.ReceiveBeginPlay`
  (bind _returnvalue (`self.K2_GetActorLocation`))
  (bind _actualdataasset (`self.ActualDataAsset`))
  (set `self.InitalLoc` (`self.K2_GetActorLocation`))
  (`TimelineComponent.SetPlayRate` (`self.MoveToTimeline`) (`MP_BossDataAsset.ProjectileFXDuration` (`self.ActualDataAsset`)))
  (bind (_direction _alpha) (`Timeline|MoveToTimeline` :!via `PlayFromStart`)
    (:`Update`
      (`self.K2_SetActorLocation` (`KismetMathLibrary.VLerp` (`self.InitalLoc`) (`self.FinalLocation`) _alpha)))
    (:`Finished`
      (bind _outhit (`KismetSystemLibrary.SphereTraceSingle` :`Start` _returnvalue :`End` _returnvalue :`Radius` 20.0 :`TraceChannel` "TraceTypeQuery1" :`DrawDebugType` "ForDuration"))
      (`GameplayStatics.ApplyDamage` (`.HitActor` (`GameplayStatics.BreakHitResult` _outhit)) (`KismetMathLibrary.Conv_IntToDouble` (`MP_BossDataAsset.AttackDamage` (`self.ActualDataAsset`))) null self)
      (for _ (range 1 (+ (`KismetMathLibrary.SelectInt` (`KismetMathLibrary.RandomIntegerInRange` (`MP_BossDataAsset.FirefliesAmountMin` _actualdataasset) (`MP_BossDataAsset.FirefliesAmountMax` _actualdataasset)) (`MP_BossDataAsset.FirefliesAmount` _actualdataasset) (`MP_BossDataAsset.bRandomFireflyAmount` _actualdataasset)) 1))
        (`|SpawnActorFromClass` "/Game/GPE/BP_Firefly.BP_Firefly_C" (`KismetMathLibrary.MakeTransform` (+ (`self.K2_GetActorLocation`) (`KismetMathLibrary.MakeVector` (`KismetMathLibrary.RandomFloatInRange` -20.0 20.0) (`KismetMathLibrary.RandomFloatInRange` -20.0 20.0) (`KismetMathLibrary.RandomFloatInRange` -20.0 20.0)))) "AdjustIfPossibleButAlwaysSpawn" "MultiplyWithRoot" null (`self.BossPhase`) null))
      (`self.K2_DestroyActor`))))

(fn `UserConstructionScript`)