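; Boss actor that hovers in place and exposes events for taking damage, AOE and ranged attacks, and death.
; A looping timer restarts a timeline that moves MainBody vertically for the hover, while the construction script attaches BodyPart1 to its spine socket.
; Combat events only set state flags, with hit and shoot pulsing briefly.
; Death waits briefly, spawns an explosion and destroys the actor.
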(event `self.ReceiveBeginPlay`
  (`self.HoverAnimation`)
  (`KismetSystemLibrary.K2_SetTimerDelegate` (delegate `HoverAnimation`) 5.0 true))

(event `HoverAnimation`
  (bind (_direction _alpha) (`Timeline|HoverTimeline` :!via `PlayFromStart`)
    (:`Update`
      (`SceneComponent.K2_SetRelativeLocation` (`self.MainBody`) (`KismetMathLibrary.MakeVector` 0.0 0.0 (`KismetMathLibrary.Lerp` -270.0 -230.0 _alpha)) false false))))

(event `GetDamage`
  (set `self.gotHit` true)
  (`KismetSystemLibrary.Delay` 0.1)
  (set `self.gotHit` false))

(event `AttackAOE`
  (set `self.isAOEAttacking` true))

(event `AttackRanged`
  (set `self.isRangedAttacking` true))

(event `ShootAttackRanged`
  (set `self.shoot` true)
  (`KismetSystemLibrary.Delay` 0.1)
  (set `self.shoot` false))

(event `Death`
  (set `self.dead` true)
  (`KismetSystemLibrary.Delay` 0.7)
  (`GameplayStatics.SpawnEmitterAtLocation` "/Game/Import/FXVarietyPack/Particles/P_ky_explosion.P_ky_explosion" (`self.K2_GetActorLocation`) (struct) (3.0 3.0 3.0))
  (`self.K2_DestroyActor`))

(fn `UserConstructionScript`
  (`SceneComponent.K2_AttachToComponent` (`self.BodyPart1`) (`self.MainBody`) "Spine_Socket" "KeepRelative" "KeepRelative" "KeepRelative" true))