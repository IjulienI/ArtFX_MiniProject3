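; BP_PuzzleRing is a puzzle switch ring that activates when a Character passes through it and reports progress to its assigned Puzzle Manager.
; On BeginPlay it creates a dynamic glow material and adds itself to the manager's switch total.
; Two overlap detectors each play a sound and set a 0.4-second flag.
; When both flags overlap, the ring activates once, changes its emissive color and calls AddPuzzleProgress.
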(event `self.ReceiveBeginPlay`
  (bind _puzzlemanagerref (`self.PuzzleManagerRef`))
  (bind _returnvalue (`PrimitiveComponent.CreateDynamicMaterialInstance` (`self.GlowRing`) 0 "/Game/GPE/Materials/MI_GlowRing.MI_GlowRing" "None"))
  (set `self.GlowDynamicMaterial` _returnvalue)
  ; Add Self to Total Switch count on the assigned Puzzle Manager
  (`/Engine/EditorBlueprintResources/StandardMacros.DoOnce` false
    (:`Completed`
      (set `/Game/GPE/BP_PuzzleManager.TotalSwitches` (+ (`/Game/GPE/BP_PuzzleManager.TotalSwitches` _puzzlemanagerref) 1) _puzzlemanagerref))))

(event `self.Dectector1.OnComponentBeginOverlap`
  (params (OverlappedComponent :type "PrimitiveComponent Object Reference") (OtherActor :type "Actor Object Reference") (OtherComp :type "PrimitiveComponent Object Reference") (OtherBodyIndex :type Integer) (bFromSweep :type Boolean) (SweepResult :type "HitResult Structure (by ref)"))
  ; Check Player has passed through
  (if (`KismetMathLibrary.ClassIsChildOf` (`GameplayStatics.GetObjectClass` OtherActor) "/Script/Engine.Character")
    (set `self.A_Activated` true)
    (`GameplayStatics.PlaySound2D` "/Game/Import/SFX/Environment/GlideRing.GlideRing" 1.0 1.0 0.0 null null)
    (`self.PlayerPassing`)
    (`KismetSystemLibrary.Delay` 0.4)
    (set `self.A_Activated` false)))

(event `self.Dectector2.OnComponentBeginOverlap`
  (params (OverlappedComponent :type "PrimitiveComponent Object Reference") (OtherActor :type "Actor Object Reference") (OtherComp :type "PrimitiveComponent Object Reference") (OtherBodyIndex :type Integer) (bFromSweep :type Boolean) (SweepResult :type "HitResult Structure (by ref)"))
  ; Check Player has passed through
  (if (`KismetMathLibrary.ClassIsChildOf` (`GameplayStatics.GetObjectClass` OtherActor) "/Script/Engine.Character")
    (set `self.B_Activated` true)
    (`GameplayStatics.PlaySound2D` "/Game/Import/SFX/Environment/GlideRing.GlideRing" 1.0 1.0 0.0 null null)
    (`self.PlayerPassing`)
    (`KismetSystemLibrary.Delay` 0.4)
    (set `self.B_Activated` false)))

(event `PlayerPassing`
  ; Check Player has passed through
  (if (`self.Inactive`)
    (if (and (`self.A_Activated`) (`self.B_Activated`))
      (`self.RingActive`))))

(event `RingActive`
  ; Activate Ring & send info to Puzzle Manager
  (`/Engine/EditorBlueprintResources/StandardMacros.DoOnce` false
    (:`Completed`
      (set `self.Inactive` false)
      (`MaterialInstanceDynamic.SetVectorParameterValue` (`self.GlowDynamicMaterial`) "EmissiveInactiveColor" (struct :`R` 0.332452 :`G` 0.693872 :`B` 1.0 :`A` 1.0))
      (`/Game/GPE/BP_PuzzleManager.AddPuzzleProgress` (`self.PuzzleManagerRef`)))))

(fn `UserConstructionScript`)