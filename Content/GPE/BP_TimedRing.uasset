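; Timed puzzle ring that counts as a switch hit when a character passes through it while active.
; Registers with its Puzzle Manager and Switch Activator, whose signals activate or deactivate it.
; Two detectors must trigger within a short window to add progress once until reset; deactivation subtracts that progress.
; A timeline fades the glow, swapping dynamic materials between blinking orange, with increasable frequency, and static blue on hit.
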(event `self.ReceiveBeginPlay`
  (bind _puzzlemanagerref (`self.PuzzleManagerRef`))
  (bind _returnvalue (`PrimitiveComponent.CreateDynamicMaterialInstance` (`self.GlowRing`) 0 "/Game/GPE/Materials/MI_GlowRing.MI_GlowRing" "None"))
  (bind _output_get (set `self.StaticGlowDynamicMaterial` _returnvalue))
  (`MaterialInstanceDynamic.SetVectorParameterValue` _output_get "EmissiveInactiveColor" (struct :`R` 0.332452 :`G` 0.693872 :`B` 1.0 :`A` 1.0))
  (bind _returnvalue_2 (`PrimitiveComponent.CreateDynamicMaterialInstance` (`self.GlowRing`) 0 "/Game/GPE/Materials/MI_TimedRing.MI_TimedRing" "None"))
  (bind _output_get_2 (set `self.BlinkingGlowDynamicMaterial` _returnvalue_2))
  (`MaterialInstanceDynamic.SetScalarParameterValue` _output_get_2 "GlowIntensity" 0.0)
  ; Add Self to Total Switch count on the assigned Puzzle Manager
  (`/Engine/EditorBlueprintResources/StandardMacros.DoOnce` false
    (:`Completed`
      (set `/Game/GPE/BP_PuzzleManager.TotalSwitches` (+ (`/Game/GPE/BP_PuzzleManager.TotalSwitches` _puzzlemanagerref) 1) _puzzlemanagerref)
      ; Add self to assigned Switch Activator
      (`KismetArrayLibrary.Array_AddUnique` (`/Game/GPE/BP_SwitchActivator.TargetSwitches` (`self.SwitchActivatorRef`)) self))))

(event `ActivateSwitch`
  (bind _blinkingglowdynamicmaterial (`self.BlinkingGlowDynamicMaterial`))
  ; Activate / Deactivate on signal from Switch Activator
  (`MaterialInstanceDynamic.SetVectorParameterValue` _blinkingglowdynamicmaterial "EmissiveInactiveColor" (struct :`R` 1.0 :`G` 0.14996 :`A` 1.0))
  (`PrimitiveComponent.SetMaterial` (`self.GlowRing`) 0 _blinkingglowdynamicmaterial)
  (set `self.IsActive` true)
  (set `self.IsHit` false)
  (bind (_direction _glowspeed) (`Timeline|LerpGlow` :!via `PlayFromStart` :!label _label)
    (:`Update`
      (`MaterialInstanceDynamic.SetScalarParameterValue` (`self.BlinkingGlowDynamicMaterial`) "GlowIntensity" (`KismetMathLibrary.Lerp` 0.0 15.0 _glowspeed))
      (`MaterialInstanceDynamic.SetScalarParameterValue` (`self.StaticGlowDynamicMaterial`) "GlowIntensity" (`KismetMathLibrary.Lerp` 0.0 15.0 _glowspeed)))
    (:`Finished`
      (if (not (`self.IsActive`))
        (`self.ResetFrequency`)))))

(event `Increase Frequency`
  (bind _returnvalue (* (`self.BlinkFrequency`) 2.0))
  ; Increase / Decrease Glow Frequency as feedback for player
  (`MaterialInstanceDynamic.SetScalarParameterValue` (`self.BlinkingGlowDynamicMaterial`) "Frequency" _returnvalue)
  (set `self.BlinkFrequency` _returnvalue))

(event `ResetFrequency`
  ; Increase / Decrease Glow Frequency as feedback for player
  (set `self.BlinkFrequency` 0.5)
  (`MaterialInstanceDynamic.SetScalarParameterValue` (`self.BlinkingGlowDynamicMaterial`) "Frequency" (`self.BlinkFrequency`)))

(event `DeactivateSwitch`
  ; Activate / Deactivate on signal from Switch Activator
  (set `self.IsActive` false)
  (if (`self.IsHit`)
    (`/Game/GPE/BP_PuzzleManager.SubstractPuzzleProgress` (`self.PuzzleManagerRef`))
    (goto _label :!via `ReverseFromEnd`)
    (else
      (goto _label :!via `ReverseFromEnd`))))

(event `self.Dectector1.OnComponentBeginOverlap`
  (params (OverlappedComponent :type "PrimitiveComponent Object Reference") (OtherActor :type "Actor Object Reference") (OtherComp :type "PrimitiveComponent Object Reference") (OtherBodyIndex :type Integer) (bFromSweep :type Boolean) (SweepResult :type "HitResult Structure (by ref)"))
  ; Activate on Overlap with Player
  (if (not (`self.IsCleared`))
    (if (`self.IsActive`)
      (if (`KismetMathLibrary.ClassIsChildOf` (`GameplayStatics.GetObjectClass` OtherActor) "/Script/Engine.Character")
        (set `self.A_Activated` true)
        (`self.PlayerPassing`)
        (`KismetSystemLibrary.Delay` 0.4)
        (set `self.A_Activated` false)))))

(event `self.Dectector2.OnComponentBeginOverlap`
  (params (OverlappedComponent :type "PrimitiveComponent Object Reference") (OtherActor :type "Actor Object Reference") (OtherComp :type "PrimitiveComponent Object Reference") (OtherBodyIndex :type Integer) (bFromSweep :type Boolean) (SweepResult :type "HitResult Structure (by ref)"))
  ; Activate on Overlap with Player
  (if (not (`self.IsCleared`))
    (if (`self.IsActive`)
      (if (`KismetMathLibrary.ClassIsChildOf` (`GameplayStatics.GetObjectClass` OtherActor) "/Script/Engine.Character")
        (set `self.B_Activated` true)
        (`self.PlayerPassing`)
        (`KismetSystemLibrary.Delay` 0.4)
        (set `self.B_Activated` false)))))

(event `PlayerPassing`
  ; Activate on Overlap with Player
  (if (and (`self.A_Activated`) (`self.B_Activated`))
    (`self.Switch Hit`)))

(event `Switch Hit`
  ; Inform Puzzle Manager of hit and lock switch
  (`/Engine/EditorBlueprintResources/StandardMacros.DoOnce` false :!label _label_2
    (:`Completed`
      (set `self.IsHit` true)
      (`MaterialInstanceDynamic.SetVectorParameterValue` (`self.BlinkingGlowDynamicMaterial`) "EmissiveInactiveColor" (struct :`R` 0.332452 :`G` 0.693872 :`B` 1.0 :`A` 1.0))
      (`PrimitiveComponent.SetMaterial` (`self.GlowRing`) 0 (`self.StaticGlowDynamicMaterial`))
      (`/Game/GPE/BP_PuzzleManager.AddPuzzleProgress` (`self.PuzzleManagerRef`)))))

(event `ResetHitEvent`
  ; Inform Puzzle Manager of hit and lock switch
  (goto _label_2 :!via `Reset`))

(fn `UserConstructionScript`)