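; Health pickup actor that passes the player data asset's HealthGain through ApplyDamage to whatever overlaps its sphere.
; A DoOnce gates the overlap, then spawns a hit effect, disables collision and hides the sprite.
; After a delay it shows the sprite and resets the gate, but sets collision to NoCollision again rather than re-enabling it.
; Tick yaws the actor toward the player like a billboard.
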(event `ResetPickUp`
  (goto _label :!via `Reset`))

(event `self.Sphere1.OnComponentBeginOverlap`
  (params (OverlappedComponent :type "PrimitiveComponent Object Reference") (OtherActor :type "Actor Object Reference") (OtherComp :type "PrimitiveComponent Object Reference") (OtherBodyIndex :type Integer) (bFromSweep :type Boolean) (SweepResult :type "HitResult Structure (by ref)"))
  (`/Engine/EditorBlueprintResources/StandardMacros.DoOnce` false :!label _label
    (:`Completed`
      (`GameplayStatics.ApplyDamage` OtherActor (`KismetMathLibrary.Conv_IntToDouble` (`MP_PlayerDataAsset.HealthGain` (`self.PlayerDataAsset`))) null self)
      (`GameplayStatics.SpawnEmitterAtLocation` "/Game/Import/FXVarietyPack/Particles/P_ky_hit3.P_ky_hit3" (`self.K2_GetActorLocation`) (struct) (1.0 1.0 1.0) false)
      (`PrimitiveComponent.SetCollisionEnabled` (`self.Sphere1`) "NoCollision")
      (`SceneComponent.SetHiddenInGame` (`self.health_Sprite`) true false)
      (`KismetSystemLibrary.Delay` 10.0)
      (`PrimitiveComponent.SetCollisionEnabled` (`self.Sphere1`) "NoCollision")
      (`SceneComponent.SetHiddenInGame` (`self.health_Sprite`) false false)
      (`self.ResetPickUp`))))

(event `self.ReceiveTick`
  (params (DeltaSeconds :type "Float (single-precision)"))
  (bind (_returnvalue_roll _returnvalue_pitch _returnvalue_yaw) (`KismetMathLibrary.BreakRotator` (`KismetMathLibrary.FindLookAtRotation` (`self.K2_GetActorLocation`) (`self.K2_GetActorLocation` (`GameplayStatics.GetPlayerCharacter` 0)))))
  (`self.K2_SetActorRotation` (`KismetMathLibrary.MakeRotator` 0.0 0.0 _returnvalue_yaw)))

(fn `UserConstructionScript`)