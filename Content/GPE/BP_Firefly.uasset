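; Homing firefly projectile for a boss attack, configured by the data asset matching its boss phase.
; On BeginPlay the phase data sets its color through a dynamic material and its speed, plus a lifetime when attack duration is nonzero.
; Tick smoothly turns it toward the player and sweeps it forward by a per-frame step not scaled by delta time.
; Any overlap or hit applies phase-defined damage and destroys it.
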(event `self.ReceiveBeginPlay`
  (bind _attackduration (`MP_BossDataAsset.AttackDuration` (`self.BossPhaseDataAsset`)))
  ; Set Boss Phase
  (set `self.BossPhaseDataAsset` (select `int` (`self.BossPhase`) :`0` "/Game/_Base/DataAssets/Boss/DA_BossPhase1.DA_BossPhase1" :`1` "/Game/_Base/DataAssets/Boss/DA_BossPhase2.DA_BossPhase2" :`2` "/Game/_Base/DataAssets/Boss/DA_BossPhase3.DA_BossPhase3" :!type "MP_BossDataAsset Object Reference"))
  ; Set Material Color
  (bind _returnvalue (`PrimitiveComponent.CreateDynamicMaterialInstance` (`self.Sphere1`) 0 "/Game/GPE/Materials/M_Firefly.M_Firefly" "None"))
  (`MaterialInstanceDynamic.SetVectorParameterValue` _returnvalue "Color" (`MP_BossDataAsset.FireflyColor` (`self.BossPhaseDataAsset`)))
  (`PrimitiveComponent.SetMaterial` (`self.Sphere1`) 0 _returnvalue)
  ; Set Speed and Life Spawn
  (set `self.Speed` (`MP_BossDataAsset.FirefliesSpeed` (`self.BossPhaseDataAsset`)))
  (if (not (== _attackduration 0.0))
    (`KismetSystemLibrary.Delay` _attackduration)
    (`self.K2_DestroyActor`)))

(event `self.ReceiveTick`
  (params (DeltaSeconds :type "Float (single-precision)"))
  ; Follow Player
  ;; Set Rotation
  (`self.K2_SetActorRotation` (`KismetMathLibrary.RInterpTo` (`self.K2_GetActorRotation`) (`KismetMathLibrary.FindLookAtRotation` (`self.K2_GetActorLocation`) (`self.K2_GetActorLocation` (`GameplayStatics.GetPlayerPawn` 0))) DeltaSeconds 4.0))
  ;; Set Location
  (`self.K2_SetActorLocation` (+ (* (`self.GetActorForwardVector`) (`self.Speed`)) (`self.K2_GetActorLocation`)) true))

(event `self.Sphere.OnComponentBeginOverlap`
  (params (OverlappedComponent :type "PrimitiveComponent Object Reference") (OtherActor :type "Actor Object Reference") (OtherComp :type "PrimitiveComponent Object Reference") (OtherBodyIndex :type Integer) (bFromSweep :type Boolean) (SweepResult :type "HitResult Structure (by ref)"))
  ; Destroy on Hit / Overlap and deal damage
  (`self.DamageActor` OtherActor))

(event `self.Sphere.OnComponentHit`
  (params (HitComponent :type "PrimitiveComponent Object Reference") (OtherActor :type "Actor Object Reference") (OtherComp :type "PrimitiveComponent Object Reference") (NormalImpulse :type "Vector Structure") (Hit :type "HitResult Structure (by ref)"))
  ; Destroy on Hit / Overlap and deal damage
  (`self.DamageActor` OtherActor))

(fn `DamageActor`
  (params (`Damaged Actor` :type "Actor Object Reference"))
  (`GameplayStatics.ApplyDamage` `Damaged Actor` (`MP_BossDataAsset.FireflyAttackDamage` (`self.BossPhaseDataAsset`)) null self)
  (`self.K2_DestroyActor`))

(fn `UserConstructionScript`)