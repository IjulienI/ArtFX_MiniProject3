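; BP_Activator is a puzzle switch that triggers a door or BPI_Puzzle target actors, such as pistons.
; A sphere overlap primes it, then it fires on Interact or, for auto-activators, when its glow timeline finishes, provided it has power.
; Manual activation of mechanisms sets a timer after a start pause, and Standalone switches force-deactivate all other activators.
; A timeline drives a shared dynamic material to show sign glow.
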(event `self.ReceiveBeginPlay`
  (bind _returnvalue (`KismetMaterialLibrary.CreateDynamicMaterialInstance` (`PrimitiveComponent.GetMaterial` (`self.SignCircle`) 0)))
  (bind _output_get (set `self.GlowRingMaterial` _returnvalue))
  (`PrimitiveComponent.SetMaterial` (`self.SignCircle`) 0 _output_get)
  (`PrimitiveComponent.SetMaterial` (`self.XSign`) 0 _output_get)
  (if (`self.SelfPowered`)
    (set `self.EnoughPower` true)
    (else
      (set `self.EnoughPower` false))))

(event `self.Sphere.OnComponentBeginOverlap`
  (params (OverlappedComponent :type "PrimitiveComponent Object Reference") (OtherActor :type "Actor Object Reference") (OtherComp :type "PrimitiveComponent Object Reference") (OtherBodyIndex :type Integer) (bFromSweep :type Boolean) (SweepResult :type "HitResult Structure (by ref)"))
  ; Activator On
  (if (`KismetSystemLibrary.DoesImplementInterface` OtherActor)
    (if (`self.EnoughPower`)
      (set `self.Ready` true)
      (if (`self.Auto Activator`)
        (`self.Activation Glow Sign` false 0.1)
        (else
          (`self.Activation Glow Sign` false 0.001)))
      (else
        (`self.Not Enough Power`)))))

(event `self.Sphere.OnComponentEndOverlap`
  (params (OverlappedComponent :type "PrimitiveComponent Object Reference") (OtherActor :type "Actor Object Reference") (OtherComp :type "PrimitiveComponent Object Reference") (OtherBodyIndex :type Integer))
  ; Activator Off
  (if (`KismetSystemLibrary.DoesImplementInterface` OtherActor)
    (set `self.Ready` false)
    (`self.ResetAutoGlowCheck`)
    (`self.Finish Glow` 0.0)))

(event `/Game/GPE/Activators/BPI_Interactable.Interact`
  (params (Interactor :type "Object Object Reference"))
  ; Manual Activation
  (if (`self.Ready`)
    (if (`self.EnoughPower`)
      (if (not (`self.IsActivated`))
        (set `self.IsActivated` true)
        (`GameplayStatics.PlaySound2D` (`self.ActivateSound`) 1.0 1.0 0.0 null null)
        (`self.Activation Glow Sign` false 0.1)
        (`self.Activate Mechanism`)
        ; Deactivate Other Activators
        (if (`self.Standalone`)
          (bind _outactors (`GameplayStatics.GetAllActorsOfClass` "BP_Activator_C"))
          (bind _output_get (set `self.OtherActivators` _outactors))
          (bind _returnvalue (`KismetArrayLibrary.Array_RemoveItem` _output_get (`|GetArrayItem` _output_get (`KismetArrayLibrary.Array_Find` _output_get self))))
          (if _returnvalue
            (for _array_element (`self.OtherActivators`)
              (if (`KismetSystemLibrary.DoesImplementInterface` _array_element "/Game/GPE/Activators/BPI_Interactable.BPI_Interactable_C")
                (`self.ForceDeactivate` _array_element))))))
      (else
        (`self.Not Enough Power`)))))

(event `Activate Mechanism`
  (bind _targetdoor (`self.TargetDoor`))
  ; Activate Mechanism
  (if (`self.TargetsDoor`)
    ;; Open Door
    (if (`KismetSystemLibrary.DoesImplementInterface` _targetdoor "/Game/GPE/BPI_Puzzle.BPI_Puzzle_C")
      (message `/Game/GPE/BPI_Puzzle.Activate` _targetdoor 0.0 0.0))
    (else
      ;; Piston Puzzle
      ;;; Activate Target Mechanisms
      (if (`self.Auto Activator`)
        (set `self.IsActivated` true)
        (for _array_element (`self.TargetActors`)
          (if (`KismetSystemLibrary.DoesImplementInterface` _array_element "/Game/GPE/BPI_Puzzle.BPI_Puzzle_C")
            (message `/Game/GPE/BPI_Puzzle.Activate` _array_element 0.0 0.0)))
        (else
          (for _array_element_2 (`self.TargetActors`)
            (if (`KismetSystemLibrary.DoesImplementInterface` _array_element_2 "/Game/GPE/BPI_Puzzle.BPI_Puzzle_C")
              (message `/Game/GPE/BPI_Puzzle.Activate` _array_element_2 0.0 (`self.Start Pause`))
              (bind _returnvalue (`KismetSystemLibrary.K2_SetTimerDelegate` (`|CreateDelegate` :!event `Deactivate Mechanism`) (+ (`self.ActivationTime`) (`self.Start Pause`))))
              (set `self.DeactivateTimer` _returnvalue))))))))

(event `ForceDeactivate`
  ; ForceDeactivate
  (`KismetSystemLibrary.K2_ClearAndInvalidateTimerHandle` (`self.DeactivateTimer`))
  (if (`self.IsActivated`)
    (for _array_element (`self.TargetActors`)
      (if (`KismetSystemLibrary.DoesImplementInterface` _array_element "/Game/GPE/BPI_Puzzle.BPI_Puzzle_C")
        (message `/Game/GPE/BPI_Puzzle.Deactivate` _array_element)))
    (set `self.IsActivated` false)
    (if (`self.Ready`)
      (`self.Finish Glow` 1.0)
      (else
        (`self.Finish Glow` 0.0)))))

(event `Deactivate Mechanism`
  ; Deactivate Mechanism
  (if (`self.IsActivated`)
    (`GameplayStatics.PlaySound2D` (`self.DeactivateSound`) 1.0 1.0 0.0 null null)
    (for _array_element (`self.TargetActors`)
      (if (`KismetSystemLibrary.DoesImplementInterface` _array_element "/Game/GPE/BPI_Puzzle.BPI_Puzzle_C")
        (message `/Game/GPE/BPI_Puzzle.Deactivate` _array_element)))
    (set `self.IsActivated` false)
    (if (`self.Ready`)
      (`self.Finish Glow` 1.0)
      (else
        (`self.Finish Glow` 0.0)))))

(event `Activation Glow Sign`
  (params (`Quick Glow` :type Boolean) (TargetGlowStrength :type "Float (double-precision)"))
  ; Glow Sign
  (set `self.TargetGlowStrength` TargetGlowStrength)
  (`self.ResetAutoGlowCheck`)
  (bind _returnvalue (`MaterialInstanceDynamic.K2_GetScalarParameterValue` (`self.GlowRingMaterial`) "Strength"))
  (set `self.CurrentGlowLevel` _returnvalue)
  (bind (_direction _glow) (`Timeline|GlowSignTimeline` :!via `PlayFromStart` :!label _label)
    (:`Update`
      (`MaterialInstanceDynamic.SetScalarParameterValue` (`self.GlowRingMaterial`) "Strength" (`KismetMathLibrary.Lerp` (`self.CurrentGlowLevel`) (`self.TargetGlowStrength`) _glow)))
    (:`Finished`
      (if (`self.Auto Activator`)
        ;; Auto Activation / Deactivation
        (`/Engine/EditorBlueprintResources/StandardMacros.DoOnce` false :!label _label_2
          (:`Completed`
            (if (`self.Ready`)
              (`self.Activate Mechanism`)
              (else
                (`self.Deactivate Mechanism`)))))))))

(event `Finish Glow`
  (params (TargetEndGlow :type "Float (double-precision)"))
  ; Glow Sign
  (set `self.CurrentGlowLevel` TargetEndGlow)
  (goto _label :!via `Reverse`))

(event `ResetAutoGlowCheck`
  ; Glow Sign
  ;; Auto Activation / Deactivation
  (goto _label_2 :!via `Reset`))

(event `Not Enough Power`)

(fn `IsAutomatic?`
  (returns (IsAutomatic :type Boolean))
  (return (`self.Auto Activator`)))

(fn `IsInteracting?`
  (returns (IsInteracting :type Boolean))
  (return (`self.IsActivated`)))

(fn `UserConstructionScript`)