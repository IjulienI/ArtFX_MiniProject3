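; BP_OnboardingGate is a puzzle gate that opens once enough switches are active.
; External add and subtract events adjust a counter, and reaching the total freezes and ends linked pressure plates or notifies a dash switch activator, depending on puzzle type.
; A one-time activation recolors the crystals' shared dynamic material, plays a sound, then after a delay slides both doors apart via a timeline.
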(event `self.ReceiveBeginPlay`
  (bind _returnvalue (`PrimitiveComponent.CreateDynamicMaterialInstance` (`self.CrystalL`) 0 "/Game/GPE/Materials/MI_Crystal.MI_Crystal" "None"))
  (bind _output_get (set `self.GlowDynamicMaterial` _returnvalue))
  (`PrimitiveComponent.SetMaterial` (`self.CrystalL`) 0 _output_get)
  (`PrimitiveComponent.SetMaterial` (`self.CrystalR`) 0 _output_get))

(event `AddPuzzleProgress`
  (set `self.SwitchesActivated` (+ (`self.SwitchesActivated`) 1))
  (`self.CheckPuzzleProgress`))

(event `SubstractPuzzleProgress`
  (set `self.SwitchesActivated` (- (`self.SwitchesActivated`) 1))
  (`self.CheckPuzzleProgress`))

(event `CheckPuzzleProgress`
  (bind _switchactivator (`self.SwitchActivator`))
  (if (>= (`self.SwitchesActivated`) (`self.TotalSwitches`))
    (`self.GateActive`)
    (if (`self.IsFloorSwitchPuzzle`)
      (for _array_element (`self.PressurePlateActors`)
        (set `/Game/GPE/BP_PressurePlate.IsFrozen` true _array_element)
        (`/Game/GPE/BP_PressurePlate.EndPuzzle` _array_element))
      (elif (`self.IsDashSwitchPuzzle`)
        (`/Engine/EditorBlueprintResources/StandardMacros.IsValid` _switchactivator
          (:`Is Valid`
            (`/Game/GPE/BP_SwitchActivator.PuzzleCleared` _switchactivator)))))))

(event `GateActive`
  (`/Engine/EditorBlueprintResources/StandardMacros.DoOnce` false
    (:`Completed`
      (`MaterialInstanceDynamic.SetVectorParameterValue` (`self.GlowDynamicMaterial`) "EmissiveInactiveColor" (struct :`R` 0.332452 :`G` 0.693872 :`B` 1.0 :`A` 1.0))
      (`GameplayStatics.PlaySound2D` null 1.0 1.0 0.0 null null)
      (`KismetSystemLibrary.Delay` 2.0)
      (bind (_direction _doortrack) (`Timeline|OpenGate` :!via `PlayFromStart`)
        (:`Update`
          (`SceneComponent.K2_SetRelativeLocation` (`self.GateDoorR`) (`KismetMathLibrary.MakeVector` _doortrack 0.0 -70.0) false false)
          (`SceneComponent.K2_SetRelativeLocation` (`self.GateDoorL`) (`KismetMathLibrary.MakeVector` (* _doortrack -1.0) 0.0 -70.0) false false))))))

(fn `UserConstructionScript`)