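; Puzzle floor switch that activates its target switches for a limited time when a Character steps on it.
; It registers with the puzzle manager, lowers its piston by timeline and recolors its glow ring through a dynamic material.
; Delays raise target frequency and swap timer components as time runs down, alongside a deactivation timer.
; Re-stepping while active restarts the targets; clearing the puzzle disables the switch and marks targets cleared.
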(event `self.ReceiveBeginPlay`
  (set `/Game/GPE/BP_PuzzleManager.SwitchActivator` self (`self.PuzzleManagerRef`))
  (bind _returnvalue (`PrimitiveComponent.CreateDynamicMaterialInstance` (`self.BoxRing`) 0 "/Game/GPE/Materials/MI_GlowPressurePlate.MI_GlowPressurePlate" "None"))
  (set `self.GlowDynamicMaterial` _returnvalue))

(event `self.Box.OnComponentBeginOverlap`
  (params (OverlappedComponent :type "PrimitiveComponent Object Reference") (OtherActor :type "Actor Object Reference") (OtherComp :type "PrimitiveComponent Object Reference") (OtherBodyIndex :type Integer) (bFromSweep :type Boolean) (SweepResult :type "HitResult Structure (by ref)"))
  (if (not (`self.IsCompleted`))
    (if (`KismetMathLibrary.ClassIsChildOf` (`GameplayStatics.GetObjectClass` OtherActor) "/Script/Engine.Character")
      (if (not (`self.IsActive`))
        (set `self.RefreshingSwitch` false)
        (`self.LowerSwitch`)
        (else
          (set `self.RefreshingSwitch` true)
          (`self.DeactivateSwitches`)
          (`KismetSystemLibrary.Delay` 0.2)
          (`self.ActivateSwitches`))))))

(event `LowerSwitch`
  (`self.ActivateSwitches`)
  (bind (_direction _pistondown) (`Timeline|SwitchDown` :!via `PlayFromStart` :!label _label)
    (:`Update`
      (`SceneComponent.K2_SetRelativeLocation` (`self.SwitchPiston`) (`KismetMathLibrary.MakeVector` 0.0 0.0 _pistondown) false false))))

(event `RaiseSwitch`
  (goto _label :!via `ReverseFromEnd`))

(event `ActivateSwitches`
  ; Activate puzzle switches and start timer
  (set `self.IsActive` true)
  (`MaterialInstanceDynamic.SetVectorParameterValue` (`self.GlowDynamicMaterial`) "EmissiveInactiveColor" (struct :`R` 0.332452 :`G` 0.693872 :`B` 1.0 :`A` 1.0))
  (for _array_element (`self.TargetSwitches`)
    (`/Game/GPE/BP_TimedRing.ActivateSwitch` _array_element)
    (`AudioComponent.Play` (`self.Timer`) 0.0))
  (`KismetSystemLibrary.Delay` (`self.Start Pause`))
  (bind _returnvalue (`KismetSystemLibrary.K2_SetTimerDelegate` (`|CreateDelegate` :!event `DeactivateSwitches`) (+ (`self.PuzzleTime`) (`self.Start Pause`))))
  (set `self.DeactivateTimer` _returnvalue)
  (`KismetSystemLibrary.Delay` (/ (`self.PuzzleTime`) 2.0))
  (for _array_element_2 (`self.TargetSwitches`)
    (`/Game/GPE/BP_TimedRing.Increase Frequency` _array_element_2)
    (`AudioComponent.Play` (`self.Timer1`) 0.0)
    (`AudioComponent.Stop` (`self.Timer`)))
  (`KismetSystemLibrary.Delay` (/ (`self.PuzzleTime`) 4.0))
  (for _array_element_3 (`self.TargetSwitches`)
    (`/Game/GPE/BP_TimedRing.Increase Frequency` _array_element_3)
    (`AudioComponent.Play` (`self.Timer2`) 0.0)
    (`AudioComponent.Stop` (`self.Timer1`))))

(event `DeactivateSwitches`
  ; Deactivate all switches and reset their event
  (`MaterialInstanceDynamic.SetVectorParameterValue` (`self.GlowDynamicMaterial`) "EmissiveInactiveColor" (struct :`R` 1.0 :`G` 0.14996 :`A` 1.0))
  (for _array_element (`self.TargetSwitches`)
    (`/Game/GPE/BP_TimedRing.DeactivateSwitch` _array_element)
    (`/Game/GPE/BP_TimedRing.ResetHitEvent` _array_element))
  (`KismetSystemLibrary.K2_ClearAndInvalidateTimerHandle` (`self.DeactivateTimer`))
  (if (`self.RefreshingSwitch`)
    (set `self.RefreshingSwitch` false)
    (else
      (`self.RaiseSwitch`)))
  (set `self.IsActive` false))

(event `PuzzleCleared`
  (set `self.IsCompleted` true)
  (`KismetSystemLibrary.K2_ClearAndInvalidateTimerHandle` (`self.DeactivateTimer`))
  (`ActorComponent.K2_DestroyComponent` (`self.Timer`))
  (`ActorComponent.K2_DestroyComponent` (`self.Timer1`))
  (`ActorComponent.K2_DestroyComponent` (`self.Timer2`))
  (for _array_element (`self.TargetSwitches`)
    (set `/Game/GPE/BP_TimedRing.IsCleared` true _array_element)))

(fn `UserConstructionScript`)