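; Actor component that respawns the player after death at a stored respawn transform.
; Respawn plays the HUD death animation and a death sound, then after a short delay zeroes velocity and cancels any wall run or dash.
; It teleports the character, turns the controller to the saved yaw and resets life on BP_BaseCharacter.
; After another short delay, it plays the death animation in reverse to reveal the game.
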(event `self.Respawn`
  (bind _returnvalue (`GameplayStatics.GetPlayerCharacter` 0))
  (bind _currentrespawntransform (`self.CurrentRespawnTransform`))
  (bind (_returnvalue_roll _returnvalue_pitch) (`KismetMathLibrary.BreakRotator` (`Controller.GetControlRotation` (`GameplayStatics.GetPlayerController` 0))))
  (bind _returnvalue_2 (`Actor.GetComponentByClass` _returnvalue "/Game/_Base/Character/Components/AC_WallRunComponent.AC_WallRunComponent_C"))
  (bind _returnvalue_3 (`Actor.GetComponentByClass` _returnvalue "/Game/_Base/Character/Components/AC_DashComponent.AC_DashComponent_C"))
  (bind _ashud_game (cast `/Game/_Base/Managers/InGame/HUD_Game` (`PlayerController.GetHUD` (`GameplayStatics.GetPlayerController` 0))))
  (bind _gameviewref (`/Game/_Base/Managers/InGame/HUD_Game.gameViewRef` _ashud_game))
  (bind _death (`/Game/_Base/UI/WBP_GameView.Death` _gameviewref))
  (`UserWidget.PlayAnimation` _gameviewref _death 0.0 1 "Forward" 1.0 false)
  (`GameplayStatics.PlaySound2D` "/Game/Import/SFX/Player/PlayerDie.PlayerDie" 1.0 1.0 0.0 null null)
  (`KismetSystemLibrary.Delay` 0.4)
  (`|ExecutionSequence`
    (:`then_0`
      (set `MovementComponent.Velocity` (0.0 0.0 0.0) (`Character.CharacterMovement` _returnvalue))
      (`/Engine/EditorBlueprintResources/StandardMacros.IsValid` _returnvalue_2
        (:`Is Valid`
          (`/Game/_Base/Character/Components/AC_WallRunComponent.ResetWallRun` _returnvalue_2))
        (:`Is Not Valid`
          _))
      (`/Engine/EditorBlueprintResources/StandardMacros.IsValid` _returnvalue_3
        (:`Is Valid`
          (`MP_DashComponent.StopDash` _returnvalue_3))
        (:`Is Not Valid`
          _))
      (`Actor.K2_SetActorLocation` (`GameplayStatics.GetPlayerCharacter` 0) (.location _currentrespawntransform) false true)
      (`Controller.SetControlRotation` (`GameplayStatics.GetPlayerController` 0) (`KismetMathLibrary.MakeRotator` _returnvalue_roll _returnvalue_pitch (.yaw (.rotation _currentrespawntransform))))
      (bind _asbp_base_character (cast `/Game/_Base/Character/BP_BaseCharacter` _returnvalue))
      (`/Game/_Base/Character/BP_BaseCharacter.ResetLife` _asbp_base_character))
    (:`then_1`
      (`KismetSystemLibrary.Delay` 0.4)
      (`UserWidget.PlayAnimation` _gameviewref _death 0.0 1 "Reverse" 1.0 false))))