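; Actor component that gives the player character wall running and wall jumping.
; While airborne, Tick traces both sides and, given enough speed, zeroes gravity, flattens velocity and overrides forward direction along the wall.
; A DoOnce snaps the player on contact and refreshes jumps and dash, while Tick interpolates mesh tilt and camera offset.
; Jumping off launches along the angled wall normal, then briefly pauses detection; tuning comes from data assets.
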(event `self.ReceiveBeginPlay`
  (bind _asbp_base_character (cast `/Game/_Base/Character/BP_BaseCharacter` (`GameplayStatics.GetPlayerCharacter` 0)))
  (set `self.playerRef` _asbp_base_character))

(event `ResetHasHitDO`
  (bind _returnvalue (`GameplayStatics.GetPlayerCharacter` 0))
  (bind _returnvalue_2 (`Actor.GetComponentByClass` (`self.GetOwner`) "/Game/_Base/Character/Components/AC_DashComponent.AC_DashComponent_C"))
  (bind _returnvalue_3 (`Actor.K2_GetActorLocation` _returnvalue))
  (bind (_bblockinghit _binitialoverlap _time _distance _location _impactpoint _normal) (`GameplayStatics.BreakHitResult` (`self.HitWall`)))
  ;[0.15 0.15 0.15 0.502] Check for walls to authorise run
  (goto _label_2 :!via `Reset`))

(event `BreakLineTrace`
  (bind _returnvalue (`GameplayStatics.GetPlayerCharacter` 0))
  (bind _returnvalue_2 (`GameplayStatics.GetPlayerCharacter` 0))
  (bind _returnvalue_3 (`Actor.GetComponentByClass` (`self.GetOwner`) "/Game/_Base/Character/Components/AC_DashComponent.AC_DashComponent_C"))
  (bind _returnvalue_4 (`Actor.K2_GetActorLocation` _returnvalue_2))
  (bind (_bblockinghit _binitialoverlap _time _distance _location _impactpoint _normal) (`GameplayStatics.BreakHitResult` (`self.HitWall`)))
  (bind _charactermovement (`Character.CharacterMovement` (`GameplayStatics.GetPlayerCharacter` 0)))
  (bind _returnvalue_5 (- (`Actor.K2_GetActorLocation` _returnvalue) (`KismetMathLibrary.MakeVector` 0.0 0.0 (`MP_WallRunDataAsset.DetectionRayZOffset` (`self.WallRunDataAsset`)))))
  (bind _gravityscale (`CharacterMovementComponent.GravityScale` (`Character.CharacterMovement` (`GameplayStatics.GetPlayerCharacter` 0))))
  (bind _returnvalue_6 (`KismetMathLibrary.SelectFloat` -1.0 1.0 (< (`KismetMathLibrary.Dot_VectorVector` (`.Normal` (`GameplayStatics.BreakHitResult` (`self.HitWall`))) (`Actor.GetActorRightVector` (`GameplayStatics.GetPlayerCharacter` 0))) 0.0)))
  (bind _returnvalue_7 (* (+ (`CapsuleComponent.CapsuleRadius` (`Character.CapsuleComponent` _returnvalue)) (`MP_WallRunDataAsset.DetectionRayWidthSize` (`self.WallRunDataAsset`))) (`Actor.GetActorRightVector` _returnvalue)))
  ;[0.15 0.15 0.15 0.502] Check for walls to authorise run
  (goto _label :!via `Break`))

(event `self.ReceiveTick`
  (params (DeltaSeconds :type "Float (single-precision)"))
  (bind _returnvalue (`GameplayStatics.GetPlayerCharacter` 0))
  (bind _returnvalue_2 (`GameplayStatics.GetPlayerCharacter` 0))
  (bind (_returnvalue_x _returnvalue_y _returnvalue_z) (`KismetMathLibrary.BreakVector` (`Actor.K2_GetActorLocation` (`GameplayStatics.GetPlayerCharacter` 0))))
  (bind _returnvalue_3 (`Actor.GetComponentByClass` (`self.GetOwner`) "/Game/_Base/Character/Components/AC_DashComponent.AC_DashComponent_C"))
  (bind _returnvalue_4 (`Actor.K2_GetActorLocation` _returnvalue_2))
  (bind (_bblockinghit _binitialoverlap _time _distance _location _impactpoint _normal) (`GameplayStatics.BreakHitResult` (`self.HitWall`)))
  (bind _charactermovement (`Character.CharacterMovement` (`GameplayStatics.GetPlayerCharacter` 0)))
  (bind _springarm (`/Game/_Base/Character/BP_BaseCharacter.SpringArm` (`self.playerRef`)))
  (bind _returnvalue_5 (- (`Actor.K2_GetActorLocation` _returnvalue) (`KismetMathLibrary.MakeVector` 0.0 0.0 (`MP_WallRunDataAsset.DetectionRayZOffset` (`self.WallRunDataAsset`)))))
  (bind (_relativerotation_roll _relativerotation_pitch _relativerotation_yaw) (`KismetMathLibrary.BreakRotator` (`SceneComponent.RelativeRotation` (`Character.Mesh` (`GameplayStatics.GetPlayerCharacter` 0)))))
  (bind _gravityscale (`CharacterMovementComponent.GravityScale` (`Character.CharacterMovement` (`GameplayStatics.GetPlayerCharacter` 0))))
  (bind (_velocity_x _velocity_y _velocity_z) (`KismetMathLibrary.BreakVector` (`MovementComponent.Velocity` (`Character.CharacterMovement` (`GameplayStatics.GetPlayerCharacter` 0)))))
  (bind _returnvalue_6 (`KismetMathLibrary.SelectFloat` -1.0 1.0 (< (`KismetMathLibrary.Dot_VectorVector` (`.Normal` (`GameplayStatics.BreakHitResult` (`self.HitWall`))) (`Actor.GetActorRightVector` (`GameplayStatics.GetPlayerCharacter` 0))) 0.0)))
  (bind _returnvalue_7 (* (+ (`CapsuleComponent.CapsuleRadius` (`Character.CapsuleComponent` _returnvalue)) (`MP_WallRunDataAsset.DetectionRayWidthSize` (`self.WallRunDataAsset`))) (`Actor.GetActorRightVector` _returnvalue)))
  ;[0.15 0.15 0.15 0.502] Check for walls to authorise run
  ;;[0 0.06662 1 0.5] Tick
  (`|ExecutionSequence`
    (:`then_0`
      (if (and (`self.IsInTheAir`) (`self.bCanCheck`) (>= _velocity_z (* (`MP_WallRunDataAsset.JumpVelBeforeWallRunStop` (`self.WallRunDataAsset`)) -1.0)) (>= _returnvalue_z (+ (`self.StartJumpFromGroundHeight`) (`MP_WallRunDataAsset.HeightBeforeWallRun` (`self.WallRunDataAsset`)))))
        (set `self.bHasHitWall` false)
        (for _index (range 2) :!label _label
          (bind (_outhit _returnvalue_8) (`KismetSystemLibrary.LineTraceSingle` :`Start` _returnvalue_5 :`End` (select `int` _index :`0` (- _returnvalue_5 _returnvalue_7) :`1` (+ _returnvalue_5 _returnvalue_7)) :`TraceChannel` "TraceTypeQuery3" :`DrawDebugType` "ForDuration"))
          (if _returnvalue_8
            (set `self.bHasHitWall` true)
            (set `self.HitWall` _outhit)
            (`self.BreakLineTrace`)
            (else
              (set `self.bHasHitWall` false))))
        (if (`self.bHasHitWall`)
          (`|ExecutionSequence`
            (:`then_0`
              (`/Engine/EditorBlueprintResources/StandardMacros.DoOnce` false :!label _label_2
                (:`Completed`
                  (`Actor.K2_SetActorLocation` _returnvalue_2 (- _returnvalue_4 (* (- (`KismetMathLibrary.VSize` (- _location _returnvalue_4)) 44.0) _normal)) true false)
                  (`self.ResetJumpCount`)
                  (`/Engine/EditorBlueprintResources/StandardMacros.IsValid` _returnvalue_3
                    (:`Is Valid`
                      (`MP_DashComponent.ResetCooldown` _returnvalue_3))))))
            (:`then_1`
              (message `/Game/_Base/Interfaces/BPI_PlayerController.OverrideForwardDirection` (`GameplayStatics.GetPlayerController` 0) (`KismetMathLibrary.RotateAngleAxis` _normal (* _returnvalue_6 -90.0) (0.0 0.0 1.0)))
              (if (>= (`KismetMathLibrary.VSize` (`self.IsRunning?`)) (+ (`MP_PlayerDataAsset.WalkSpeed` (`self.PlayerDataAsset`)) 50.0))
                (message `/Game/_Base/Interfaces/BPI_PlayerController.SetIsOnWall` (`GameplayStatics.GetPlayerController` 0) true)
                (set `CharacterMovementComponent.FallingLateralFriction` 1.0 _charactermovement)
                (set `CharacterMovementComponent.GravityScale` 0.0 _charactermovement)
                (set `MovementComponent.Velocity` (`KismetMathLibrary.MakeVector` (.x (`self.IsRunning?`)) (.y (`self.IsRunning?`))) _charactermovement)
                (set `self.CharacterPitchCurrentTilt` (* (`MP_WallRunDataAsset.CharacterMeshTiltAngle` (`self.WallRunDataAsset`)) _returnvalue_6))
                (set `self.TargetSocketLocation` (* (`KismetMathLibrary.InverseTransformDirection` (`Actor.GetTransform` (`self.playerRef`)) (`.Normal` (`GameplayStatics.BreakHitResult` (`self.HitWall`)))) (`MP_WallRunDataAsset.CameraOffsetWallRun` (`self.WallRunDataAsset`))))
                (else
                  (message `/Game/_Base/Interfaces/BPI_PlayerController.SetIsOnWall` (`GameplayStatics.GetPlayerController` 0) false :!label _label_3)
                  (set `CharacterMovementComponent.GravityScale` (`KismetMathLibrary.SelectFloat` _gravityscale (`MP_PlayerDataAsset.GravityScale` (`self.PlayerDataAsset`)) (!= _gravityscale 0.0)) (`Character.CharacterMovement` (`GameplayStatics.GetPlayerCharacter` 0)))
                  (set `CharacterMovementComponent.FallingLateralFriction` 0.0 (`Character.CharacterMovement` (`GameplayStatics.GetPlayerCharacter` 0)))
                  (set `self.CharacterPitchCurrentTilt` 0.0)
                  (`self.ResetHasHitDO`)
                  (set `self.TargetSocketLocation` (`MP_PlayerDataAsset.SocketOffset` (`self.PlayerDataAsset`)))))))
          (else
            (goto _label_3)))))
    (:`then_1`
      ;[0.15 0.15 0.15 0.502] TICK - Rotate player mesh
      (`SceneComponent.K2_SetRelativeRotation` (`Character.Mesh` (`GameplayStatics.GetPlayerCharacter` 0)) (`KismetMathLibrary.MakeRotator` 0.0 (`KismetMathLibrary.FInterpTo` _relativerotation_pitch (`self.CharacterPitchCurrentTilt`) (`GameplayStatics.GetWorldDeltaSeconds`) 10.0) _relativerotation_yaw) false false)
      (set `SpringArmComponent.SocketOffset` (`KismetMathLibrary.VInterpTo` (`SpringArmComponent.SocketOffset` _springarm) (`self.TargetSocketLocation`) (`GameplayStatics.GetWorldDeltaSeconds`) (`MP_WallRunDataAsset.CameraOffsetInterpSpeed` (`self.WallRunDataAsset`))) _springarm))))

(event `ResetWallRun`
  ; Reset Wall run
  (message `/Game/_Base/Interfaces/BPI_PlayerController.SetIsOnWall` (`GameplayStatics.GetPlayerController` 0) false)
  (set `CharacterMovementComponent.GravityScale` (`MP_PlayerDataAsset.GravityScale` (`self.PlayerDataAsset`)) (`Character.CharacterMovement` (`GameplayStatics.GetPlayerCharacter` 0)))
  (set `self.CharacterPitchCurrentTilt` 0.0)
  (`self.ResetHasHitDO`)
  (set `self.TargetSocketLocation` (`MP_PlayerDataAsset.SocketOffset` (`self.PlayerDataAsset`)))
  (set `self.bCanCheck` false)
  (`KismetSystemLibrary.RetriggerableDelay` 0.2)
  (set `self.bCanCheck` true))

(event `self.JumpOfWall`
  (bind _returnvalue (`Actor.GetComponentByClass` (`self.GetOwner`) "/Game/_Base/Character/Components/AC_DashComponent.AC_DashComponent_C"))
  (bind (_bblockinghit _binitialoverlap _time _distance _location _impactpoint _normal) (`GameplayStatics.BreakHitResult` (`self.HitWall`)))
  (bind _returnvalue_2 (* (`KismetMathLibrary.RotateAngleAxis` _normal (* (`MP_WallRunDataAsset.JumpOfWallUpAngleDirection` (`self.WallRunDataAsset`)) -1.0) (`KismetMathLibrary.MakeVector` (* (.y _normal) -1.0) (.x _normal))) (`MP_WallRunDataAsset.JumpForce` (`self.WallRunDataAsset`))))
  ; Jump of Wall
  (bind _isonwall (message `/Game/_Base/Interfaces/BPI_PlayerController.GetIsOnWall` (`GameplayStatics.GetPlayerController` 0)))
  (if _isonwall
    (`Character.LaunchCharacter` (`GameplayStatics.GetPlayerCharacter` 0) _returnvalue_2 false false)
    (`KismetSystemLibrary.DrawDebugArrow` _location (+ _location _returnvalue_2) 10.0 (struct :`R` 0.002514 :`G` 0.237988 :`B` 1.0 :`A` 1.0) 10.0 1.0)
    (`self.ResetJumpCount`)
    (`self.ResetWallRun`)
    (`/Engine/EditorBlueprintResources/StandardMacros.IsValid` _returnvalue
      (:`Is Valid`
        (`MP_DashComponent.ResetCooldown` _returnvalue)))))

(fn `IsInTheAir`
  (returns (ReturnValue :type Boolean))
  (return (not (`NavMovementComponent.IsMovingOnGround` (`Character.CharacterMovement` (`GameplayStatics.GetPlayerCharacter` 0))))))

(fn `IsRunning?`
  (returns (VelocityXY :type "Vector Structure") (isSpeedEnough :type Boolean))
  (bind _charactermovement (`Character.CharacterMovement` (`GameplayStatics.GetPlayerCharacter` 0)))
  (bind (_velocity_x _velocity_y) (`KismetMathLibrary.BreakVector` (`MovementComponent.Velocity` _charactermovement)))
  (return (`KismetMathLibrary.MakeVector` _velocity_x _velocity_y) (`KismetMathLibrary.NearlyEqual_FloatFloat` (`CharacterMovementComponent.MaxWalkSpeed` _charactermovement) (`MP_PlayerDataAsset.RunSpeed` (`self.PlayerDataAsset`)))))