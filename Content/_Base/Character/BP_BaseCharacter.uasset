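; Base character Blueprint that handles life, healing, respawn and dash feedback.
; Tick watches the dash component, firing controller rumble and showing the ghost-step effect once per dash, then hiding it after a short delay.
; AnyDamage treats causers tagged "Heal" as healing capped at the data asset's max life; other damage lowers life and triggers the respawn component at zero.
; ResetLife restores maximum life.
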(event `self.ReceiveTick`
  (params (DeltaSeconds :type "Float (single-precision)"))
  (bind _ns_ghoststep (`self.NS_GhostStep`))
  (`MP_DashComponent.bInDash` (`self.AC_DashComponent`)
    (:`then`
      (`/Engine/EditorBlueprintResources/StandardMacros.DoOnce` false :!label _label
        (:`Completed`
          (`PlayerController.K2_ClientPlayForceFeedback` (`GameplayStatics.GetPlayerController` 0) "/Game/GameFeel/Haptics/FFE_Dash.FFE_Dash" "None" false false false)
          (`SceneComponent.SetVisibility` _ns_ghoststep true false))))
    (:`else`
      (`KismetSystemLibrary.Delay` 0.1)
      (`SceneComponent.SetVisibility` _ns_ghoststep false false)
      (goto _label :!via `Reset`))))

(event `self.ReceiveAnyDamage`
  (params (Damage :type "Float (single-precision)") (DamageType :type "DamageType Object Reference") (InstigatedBy :type "Controller Object Reference") (DamageCauser :type "Actor Object Reference"))
  (bind _maxlife (`MP_PlayerDataAsset.MaxLife` (`self.PlayerDataAsset`)))
  (if (not (`self.ActorHasTag` DamageCauser "Heal"))
    (bind _output_get (set `self.CurrentLife` (- (`self.CurrentLife`) Damage)))
    (if (<= _output_get 0)
      (`MP_RespawnComponent.Respawn` (`self.AC_RespawnComponent`)))
    (else
      (bind _output_get_2 (set `self.CurrentLife` (+ (`self.CurrentLife`) Damage)))
      (if (> _output_get_2 _maxlife)
        (set `self.CurrentLife` _maxlife)))))

(event `ResetLife`
  (set `self.CurrentLife` (`MP_PlayerDataAsset.MaxLife` (`self.PlayerDataAsset`))))

(fn `UserConstructionScript`)